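; BP_PuppetController is a small controller Blueprint that holds a reference to the Vanquish character.
; WaitForDodgeEnd clears that character's dodging status, with no delay inside the function itself.
; GetScreenBoundaries holds unconnected checks comparing the player camera's X and Z offset from the character against fixed limits, so it has no effect.
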(fn `UserConstructionScript`)

(fn `Wait for Dodge End`
  (`VanquishCharacter.SetDodgingStatus` (`self.VanquishCharRef`) false))