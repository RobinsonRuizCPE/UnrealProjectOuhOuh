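; Player controller for the Vanquish character, turning Enhanced Input into spline-offset movement, dodging, weapon fire, sword attacks and pausing.
; Movement and dodge feed the follow-spline component, with ability flags gating both and a timeline driving the dodge burst, afterimage effect and short cooldown.
; Aim input nudges the mouse cursor within the viewport, firing forwards to the player pawn, and sword presses re-arm shortly after release.
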(event `EnhancedInput|/Game/Characters/VanquishCharacter/Input/Actions/IA_Move`
  (params (ActionValue :type "Vector2D Structure") (ElapsedSeconds :type "Float (double-precision)") (TriggeredSeconds :type "Float (double-precision)") (InputAction :type "InputAction Object Reference" :default "/Game/Characters/VanquishCharacter/Input/Actions/IA_Move.IA_Move"))
  (bind (_lastmovementinputs_x _lastmovementinputs_y) (`KismetMathLibrary.BreakVector` (`self.LastMovementInputs`)))
  (bind _vanquishcharref (`self.VanquishCharRef`))
  (bind _returnvalue (`VanquishCharacter.HasAbilityFlag` _vanquishcharref "CanMove"))
  (bind _playerfollowsplinecomponent (`VanquishCharacter.PlayerFollowSplineComponent` _vanquishcharref))
  ;[0.05098 0.05098 0.05098] Movement
  (:`Triggered`
    (if _returnvalue
      (`PlayerFollowSplineComponent.AddHorizontalOffset` _playerfollowsplinecomponent ActionValue_X)
      (`PlayerFollowSplineComponent.AddVerticalOffset` _playerfollowsplinecomponent ActionValue_Y)
      (set `self.LastMovementInputs` (`KismetMathLibrary.MakeVector` ActionValue_X ActionValue_Y))))
  (:`Completed`
    (if _returnvalue
      (`PlayerFollowSplineComponent.AddHorizontalOffset` _playerfollowsplinecomponent (/ _lastmovementinputs_x 2.0))
      (`PlayerFollowSplineComponent.AddVerticalOffset` _playerfollowsplinecomponent (/ _lastmovementinputs_y 2.0))
      (`PlayerFollowSplineComponent.AddHorizontalOffset` _playerfollowsplinecomponent 0.0)
      (`PlayerFollowSplineComponent.AddVerticalOffset` _playerfollowsplinecomponent 0.0))))

(event `EnhancedInput|/Game/Characters/VanquishCharacter/Input/Actions/IA_Pause`
  (params (ActionValue :type Boolean) (ElapsedSeconds :type "Float (double-precision)") (TriggeredSeconds :type "Float (double-precision)") (InputAction :type "InputAction Object Reference" :default "/Game/Characters/VanquishCharacter/Input/Actions/IA_Pause.IA_Pause"))
  (:`Started`
    (`KismetSystemLibrary.PrintString` "CONTROLLER PAUSED")
    (if (not (`self.IsGamePaused`))
      (`GameplayStatics.SetGamePaused` true)
      (set `self.IsGamePaused` true)
      (bind _returnvalue (`|CreateWidget` "/Game/UI/PauseMenu/UIW_PauseMenu.UIW_PauseMenu_C" (`GameplayStatics.GetPlayerController` 0)))
      (`UserWidget.AddToViewport` _returnvalue 0))))

(event `EnhancedInput|/Game/Characters/VanquishCharacter/Input/Actions/IA_FireHeatWeapon`
  (params (ActionValue :type Boolean) (ElapsedSeconds :type "Float (double-precision)") (TriggeredSeconds :type "Float (double-precision)") (InputAction :type "InputAction Object Reference" :default "/Game/Characters/VanquishCharacter/Input/Actions/IA_FireHeatWeapon.IA_FireHeatWeapon"))
  ;[1 1 1] Right Hand Fire
  (:`Started`
    (bind _asbpplayer_pawn (cast `/Game/Characters/VanquishCharacter/Blueprints/BPPlayerPawn` (`self.VanquishCharRef`)))
    (`/Game/Characters/VanquishCharacter/Blueprints/BPPlayerPawn.FireHeatWeapon` _asbpplayer_pawn)))

(event `EnhancedInput|/Game/Characters/VanquishCharacter/Input/Actions/IA_FireRightWeapon`
  (params (ActionValue :type Boolean) (ElapsedSeconds :type "Float (double-precision)") (TriggeredSeconds :type "Float (double-precision)") (InputAction :type "InputAction Object Reference" :default "/Game/Characters/VanquishCharacter/Input/Actions/IA_FireRightWeapon.IA_FireRightWeapon"))
  ;[1 1 1] Right Hand Fire
  (:`Started`
    (bind _asbpplayer_pawn (cast `/Game/Characters/VanquishCharacter/Blueprints/BPPlayerPawn` (`self.VanquishCharRef`) :!label _label))
    (`/Game/Characters/VanquishCharacter/Blueprints/BPPlayerPawn.FireRightHand` _asbpplayer_pawn ActionValue))
  (:`Completed`
    (goto _label)))

(event `EnhancedInput|/Game/Characters/VanquishCharacter/Input/Actions/IA_Dodge`
  (params (ActionValue :type Boolean) (ElapsedSeconds :type "Float (double-precision)") (TriggeredSeconds :type "Float (double-precision)") (InputAction :type "InputAction Object Reference" :default "/Game/Characters/VanquishCharacter/Input/Actions/IA_Dodge.IA_Dodge"))
  (bind (_lastmovementinputs_x _lastmovementinputs_y) (`KismetMathLibrary.BreakVector` (`self.LastMovementInputs`)))
  (bind _vanquishcharref (`self.VanquishCharRef`))
  (bind _vanquishcharref_2 (`self.VanquishCharRef`))
  (bind _returnvalue (`self.GetComponentByClass` _vanquishcharref_2 "/Script/MyProject.PlayerFollowSplineComponent"))
  (bind (_returnvalue_x _returnvalue_y) (`KismetMathLibrary.BreakVector` (* (`KismetMathLibrary.Normal` (`KismetMathLibrary.MakeVector` _lastmovementinputs_x _lastmovementinputs_y)) (* (`GameplayStatics.GetWorldDeltaSeconds`) (`self.DodgeSpeed`)))))
  ;[1 1 1] Dodge
  (:`Started`
    (if (`VanquishCharacter.HasAbilityFlag` _vanquishcharref "CanDodge")
      (`VanquishCharacter.RemoveAbilityFlags` _vanquishcharref (`|MakeArray` "CanDodge" "CanMove" "CanMeleeAttack" :!type "ECharacterAbilityFlags Enum"))
      (`VanquishCharacter.SetDodgingStatus` _vanquishcharref true)
      (bind _returnvalue_2 (`AddComponent|NODE_AddNiagaraComponent-0` :`self` _vanquishcharref))
      (`NiagaraComponent.SetAsset` _returnvalue_2 "/Game/Characters/VanquishCharacter/VFX/NSAfterImage.NSAfterImage" true)
      (`Timeline|Timeline` :`NewTime` 1.0 :!via `PlayFromStart`
        (:`Update`
          (`PlayerFollowSplineComponent.AddHorizontalOffset` _returnvalue _returnvalue_x)
          (`PlayerFollowSplineComponent.AddVerticalOffset` _returnvalue _returnvalue_y))
        (:`Finished`
          (`VanquishCharacter.SetDodgingStatus` _vanquishcharref_2 false)
          (`VanquishCharacter.AddAbilityFlags` _vanquishcharref_2 (`|MakeArray` "CanMove" "CanMeleeAttack" :!type "ECharacterAbilityFlags Enum"))
          (`KismetSystemLibrary.Delay` 0.2)
          (`VanquishCharacter.AddAbilityFlags` _vanquishcharref_2 (`|MakeArray` "CanDodge" :!type "ECharacterAbilityFlags Enum"))
          (`ActorComponent.K2_DestroyComponent` _returnvalue_2))))))

(event `EnhancedInput|/Game/Characters/VanquishCharacter/Input/Actions/IA_Aim`
  (params (ActionValue :type "Vector2D Structure") (ElapsedSeconds :type "Float (double-precision)") (TriggeredSeconds :type "Float (double-precision)") (InputAction :type "InputAction Object Reference" :default "/Game/Characters/VanquishCharacter/Input/Actions/IA_Aim.IA_Aim"))
  (bind (_locationx _locationy) (`self.GetMousePosition`))
  (bind (_returnvalue_x _returnvalue_y) (`KismetMathLibrary.BreakVector2D` (`WidgetLayoutLibrary.GetViewportSize`)))
  (bind _thumbsticksensitivity (`self.ThumbstickSensitivity`))
  (:`Triggered`
    (`self.SetMouseLocation` (`KismetMathLibrary.FTrunc` (`KismetMathLibrary.FClamp` (+ _locationx (* ActionValue_X _thumbsticksensitivity)) 1.0 _returnvalue_x)) (`KismetMathLibrary.FTrunc` (`KismetMathLibrary.FClamp` (+ _locationy (* ActionValue_Y _thumbsticksensitivity)) 1.0 _returnvalue_y)))))

(event `EnhancedInput|/Game/Characters/VanquishCharacter/Input/Actions/IA_SwordAttack`
  (params (ActionValue :type Boolean) (ElapsedSeconds :type "Float (double-precision)") (TriggeredSeconds :type "Float (double-precision)") (InputAction :type "InputAction Object Reference" :default "/Game/Characters/VanquishCharacter/Input/Actions/IA_SwordAttack.IA_SwordAttack"))
  ;[1 1 1] SwordAttack
  (:`Started`
    (if (`self.CanBufferNextAttack`)
      (`VanquishCharacter.TriggerSwordAttack` (`self.VanquishCharRef`))
      (set `self.CanBufferNextAttack` false)))
  (:`Completed`
    (`KismetSystemLibrary.Delay` 0.2)
    (set `self.CanBufferNextAttack` true)))

(event `self.ReceiveBeginPlay`
  (bind (_returnvalue_x _returnvalue_y) (`KismetMathLibrary.BreakVector2D` (/ (`WidgetLayoutLibrary.GetViewportSize`) 2.0)))
  ;[1 1 1] Begin
  (bind _asvanquish_character (cast `VanquishCharacter` (`GameplayStatics.GetPlayerPawn` 0))
    (:`then`
      (set `self.VanquishCharRef` _asvanquish_character)
      (`self.SetMouseLocation` (`KismetMathLibrary.FTrunc` _returnvalue_x) (`KismetMathLibrary.FTrunc` _returnvalue_y)))
    (:`CastFailed`
      (`KismetSystemLibrary.PrintString` "PlayerController:cast failed"))))

(fn `UserConstructionScript`)