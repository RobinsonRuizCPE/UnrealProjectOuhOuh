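; Trigger volume that changes the horizontal and vertical offset limits of the player pawn's follow-spline component when the player overlaps its box.
; With gradual change enabled, it captures the current limits and a timeline lerps them to the new values, with play rate scaled so the blend takes the configured time.
; Otherwise it applies the new limits immediately.
; Each overlap also prints the overlapping actor's class name.
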(event `self.ReceiveActorBeginOverlap`
  (params (OtherActor :type "Actor Object Reference")))

(event `self.Box.OnComponentBeginOverlap`
  (params (OverlappedComponent :type "PrimitiveComponent Object Reference") (OtherActor :type "Actor Object Reference") (OtherComp :type "PrimitiveComponent Object Reference") (OtherBodyIndex :type Integer) (bFromSweep :type Boolean) (SweepResult :type "HitResult Structure (by ref)"))
  (`KismetSystemLibrary.PrintString` (`KismetSystemLibrary.GetClassDisplayName` (`GameplayStatics.GetObjectClass` OtherActor)))
  (bind _asbpplayer_pawn (cast `/Game/Characters/VanquishCharacter/Blueprints/BPPlayerPawn` OtherActor))
  (if (`self.GradualChange`)
    (bind _playerfollowsplinecomponent (`VanquishCharacter.PlayerFollowSplineComponent` _asbpplayer_pawn))
    (set `self.BaseHorizontalLimit` (`PlayerFollowSplineComponent.horizontal_offset_limit` _playerfollowsplinecomponent))
    (set `self.BaseVericalLimit` (`PlayerFollowSplineComponent.vertical_offset_limit` _playerfollowsplinecomponent))
    (`TimelineComponent.SetPlayRate` (`self.Timeline`) (/ 1.0 (`self.GradualChangeTime`)))
    (bind (_direction _newtrack_0) (`Timeline|Timeline` :!via `PlayFromStart`)
      (:`Update`
        (`PlayerFollowSplineComponent.SetPlayerOffsetsLimits` _playerfollowsplinecomponent (`KismetMathLibrary.Lerp` (`self.BaseHorizontalLimit`) (`self.New horizontal Limit`) _newtrack_0) (`KismetMathLibrary.Lerp` (`self.BaseVericalLimit`) (`self.New vertical Limit`) _newtrack_0))))
    (else
      (`PlayerFollowSplineComponent.SetPlayerOffsetsLimits` _playerfollowsplinecomponent (`self.New horizontal Limit`) (`self.New vertical Limit`)))))

(fn `UserConstructionScript`)