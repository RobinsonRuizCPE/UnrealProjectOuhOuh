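; Heat laser weapon actor that keeps its beam visual in line with the laser's current end point.
; Each Tick stretches LaserMesh along Z to the distance between the Muzzle socket and that end point, divided by 100.
; It also turns the whole actor toward the end point using a look-at rotation combined with a fixed 90-degree offset.
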(event `self.ReceiveBeginPlay`)

(event `self.ReceiveTick`
  (params (DeltaSeconds :type "Float (single-precision)"))
  (`SceneComponent.SetRelativeScale3D` (`self.LaserMesh`) (`KismetMathLibrary.MakeVector` 1.0 1.0 (/ (+ (`KismetMathLibrary.Vector_Distance` (`SceneComponent.GetSocketLocation` (`self.MeshComp`) "Muzzle") (`self.GetLaserCurrentEndPoint`)) 0.0) 100.0)))
  (`self.K2_SetActorRotation` (`KismetMathLibrary.ComposeRotators` (struct :`Yaw` -90.0) (`KismetMathLibrary.FindLookAtRotation` (`self.K2_GetActorLocation`) (`self.GetLaserCurrentEndPoint`)))))

(fn `UserConstructionScript`)