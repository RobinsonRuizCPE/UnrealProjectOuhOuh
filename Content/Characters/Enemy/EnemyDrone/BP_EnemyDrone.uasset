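; Flying enemy drone that chases the player along their spline and reports its kill when destroyed.
; Its follow update uses a NavigationVolume3D to path toward a point ahead of the player, drawing debug spheres along the route.
; It steers to one waypoint at a time with axis-separated velocity, re-pathing when close.
; Without a volume it uses the standard follow update; an exhausted path triggers the next-action decision.
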(event `self.ReceiveBeginPlay`)

(event `self.ReceiveTick`
  (params (DeltaSeconds :type "Float (single-precision)")))

(event `self.ReceiveDestroyed`
  (`self.UpdateEnemyKilled`))

(event `self.UpdateFollowPlayerNavMesh`
  (params (DeltaTime :type "Float (single-precision)"))
  (bind _returnvalue (`self.K2_GetActorLocation`))
  (bind _currentinterpolatedpath (`self.CurrentInterpolatedPath`))
  ;[1 1 1] Flying Logic
  (bind _asvanquish_character (cast `VanquishCharacter` (`self.PlayerTarget`)))
  (bind _returnvalue_2 (`GameplayStatics.GetActorOfClass` "/Script/Navigation3D.NavigationVolume3D")) ; Find the Navigation Volume 3D
  (set `self.NavigationVolume3D` _returnvalue_2)
  (bind _navigationvolume3d (`self.NavigationVolume3D`)
    (:`then`
      (if (`self.CanUpdateNavmeshPath`)
        (bind (_returnvalue_location _returnvalue_rotation) (`KismetMathLibrary.BreakTransform` (`VanquishCharacter.GetCurrentTransformAlongSpline` _asvanquish_character)))
        (bind (_out_path _returnvalue_3) (`NavigationVolume3D.FindPath` _navigationvolume3d (`self.K2_GetActorLocation`) (+ _returnvalue_location (* (`KismetMathLibrary.GetForwardVector` _returnvalue_rotation) 700.0)) (`|MakeArray` "ObjectTypeQuery1" "ObjectTypeQuery1" "ObjectTypeQuery1" "ObjectTypeQuery11" "ObjectTypeQuery12" "ObjectTypeQuery1" "ObjectTypeQuery1" "ObjectTypeQuery1" "ObjectTypeQuery1" :!type "EObjectTypeQuery Enum") "/Script/Engine.Actor")) ; Find a path from ourself to our destination
        (if _returnvalue_3
          (bind _output_get (set `self.Path` _out_path))
          (for _array_element _output_get
            (`KismetSystemLibrary.DrawDebugSphere` _array_element 25.0 10 (struct :`R` 1.0 :`G` 0.015096 :`A` 1.0) 1.0 1.0))
          ;;[1 1 1] Fly along the path
          (if (<= (`self.PathIndex`) (`KismetArrayLibrary.Array_LastIndex` (`self.Path`)))
            (set `self.CurrentInterpolatedPath` (`|GetArrayItem` (`self.Path`) (`self.PathIndex`)))
            (set `self.CanUpdateNavmeshPath` false)
            (else
              (`self.DecideNextAction`))))
        (else
          (set `MovementComponent.Velocity` (`self.ComputeAxisSeparatedOffsetVelocity` _returnvalue _currentinterpolatedpath (- _returnvalue _currentinterpolatedpath) (0.0 0.0) 0.0 (`self.ForwardCorrectionSpeed`)) (`self.CharacterMovement`))
          (bind _returnvalue_4 (`self.CheckDistanceToGoal` (`self.CurrentInterpolatedPath`) 200.0))
          (set `self.CanUpdateNavmeshPath` _returnvalue_4)
          (if _returnvalue_4
            (set `self.PathIndex` 1)))))
    (:`else`
      (`self.UpdateFollowPlayer` DeltaTime))))

(fn `UserConstructionScript`)