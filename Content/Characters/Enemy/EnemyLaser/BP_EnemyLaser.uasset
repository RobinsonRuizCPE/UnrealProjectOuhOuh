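; Enemy laser character Blueprint that drives the visual beam mesh for the enemy's laser attack.
; Every Tick it stretches a thin static mesh along its local Z to the distance between the CanonMuzzle socket and the current laser end point, plus an extra box extent.
; The mesh is visible only while IsFiringLaser is true; firing and end-point logic are not defined in this graph.
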(event `self.ReceiveTick`
  (params (DeltaSeconds :type "Float (single-precision)"))
  (bind _staticmesh (`self.StaticMesh`))
  (`SceneComponent.SetRelativeScale3D` _staticmesh (`KismetMathLibrary.MakeVector` 0.05 0.05 (/ (+ (`KismetMathLibrary.Vector_Distance` (`SceneComponent.GetSocketLocation` (`self.Mesh`) "CanonMuzzle") (`self.GetLaserCurrentEndPoint`)) (`self.GetAdditionalBoxExtentOverride`)) 1000.0)))
  (`SceneComponent.SetVisibility` _staticmesh (`self.IsFiringLaser`) false))

(fn `UserConstructionScript`)